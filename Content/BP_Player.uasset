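; BP_Player is a player-controlled ball that rolls and jumps through physics impulses applied to its Sphere component.
; Horizontal and vertical axis inputs share one impulse node that turns axis values into ground-plane pushes scaled by Speed.
; A motion axis event does the same using the controller's rotation rate, with X and Y swapped, despite its accelerometer label.
; Jump applies a fixed upward impulse on press, without a grounded check.
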(event `InputAxis|HorizontalInput`
  (params (AxisValue :type "Float (single-precision)"))
  ;[1 1 1] Move a ball on the ground
  (`PrimitiveComponent.AddImpulse` (`self.Sphere`) (* (`KismetMathLibrary.MakeVector` (stale `InputAxis|VerticalInput` AxisValue) AxisValue) (`self.Speed`)) "None" false :!label _label))

(event `InputAxis|AcceleroMeterInputVerticalInput`
  (params (AxisValue :type "Float (single-precision)"))
  (bind (_tilt _rotationrate) (`PlayerController.GetInputMotionState` (`GameplayStatics.GetPlayerController` 0)))
  ;[1 1 1] Accelerometer move a ball
  (`PrimitiveComponent.AddImpulse` (`self.Sphere`) (* (`KismetMathLibrary.MakeVector` (.y _rotationrate) (.x _rotationrate)) (`self.Speed`)) "None" false))

(event `InputAxis|VerticalInput`
  (params (AxisValue :type "Float (single-precision)"))
  ;[1 1 1] Move a ball on the ground
  (goto _label))

(event `InputAction|JumpInput`
  (params (Key :type "Key Structure"))
  ;[1 1 1] Jump a ball
  (:`Pressed`
    (`PrimitiveComponent.AddImpulse` (`self.Sphere`) (0.0 0.0 50000.0) "None" false)))

(fn `UserConstructionScript`)