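; Game mode that tracks pickup points and shows a win message once all pickups are collected.
; On BeginPlay it creates the BP_GameUI widget, adds it to the viewport and resets the score.
; UpdatePoints increments the score, pushes it to the widget, then calls EndGame, which makes the win text visible at a hardcoded threshold.
; ResetGame zeroes only the points, as the node hiding the win text is disconnected.
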(event `self.ReceiveBeginPlay`
  ;[1 1 1] Create a new instance of the UI and add it to the sceen
  (bind _returnvalue (`|CreateWidget` "/Game/BP_GameUI.BP_GameUI_C"))
  (bind _output_get (set `self.CurrentUI` _returnvalue))
  (`UserWidget.AddToViewport` _output_get 0)
  (`self.Reset Game`))

(event `Reset Game`
  ;[1 1 1] Reset the points and "turn off" you win message
  (set `self.CurrentPoints` 0)
  (set `/Game/BP_GameUI.Points` 0 (`self.CurrentUI`)))

(event `Update Points`
  ;[1 1 1] Increment points by 1 and update UI
  (bind _output_get (set `self.CurrentPoints` (+ (`self.CurrentPoints`) 1)))
  (set `/Game/BP_GameUI.Points` _output_get (`self.CurrentUI`))
  (`self.End Game`))

(event `End Game`
  ;[1 1 1] Check to see if all pickups are collected
  (if (>= (`self.CurrentPoints`) 8)
    (set `/Game/BP_GameUI.YouWinOpacity` 1.0 (`self.CurrentUI`))))

(fn `UserConstructionScript`)