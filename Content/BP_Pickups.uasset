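; BP_Pickups is a collectible pickup actor that spins continuously and awards points when the player touches it.
; Tick rotates it by configurable roll, pitch and yaw speeds scaled by delta time.
; On overlap with BP_Player it destroys itself, then tells BP_MyGameMode to update the points.
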(event `self.ReceiveTick`
  (params (DeltaSeconds :type "Float (single-precision)"))
  ;[1 1 1] Rotate cube
  (`self.K2_AddActorLocalRotation` (* (`KismetMathLibrary.MakeRotator` (`self.RollSpeed`) (`self.PitchSpeed`) (`self.YawnSpeed`)) DeltaSeconds)))

(event `self.ReceiveActorBeginOverlap`
  (params (OtherActor :type "Actor Object Reference"))
  ;[1 1 1] If player touches this, destroy it TODO add a point later
  (cast `/Game/BP_Player` OtherActor)
  (`self.K2_DestroyActor`)
  (bind _asbp_my_game_mode (cast `/Game/BP_MyGameMode` (`GameplayStatics.GetGameMode`)))
  (`/Game/BP_MyGameMode.Update Points` _asbp_my_game_mode))

(fn `UserConstructionScript`)